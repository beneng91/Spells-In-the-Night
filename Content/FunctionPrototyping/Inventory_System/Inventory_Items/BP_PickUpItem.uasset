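; BP_PickUpItem is a prototype inventory pickup actor whose look is driven by its item Name enum.
; On BeginPlay, GetRowNameFromEnum maps Grass or Rock to a DT_InventoryItem row, whose mesh and material are applied to the Cube.
; Box overlap only casts to BP_GameInstance.
; The loop meant to increase matching inventory quantities is disconnected and has an invalid enum input, so pickup does nothing yet.
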(event OnComponentBeginOverlap(Box)
  (params (OverlappedComponent :type Primitive%20Component%20Object%20Reference) (OtherActor :type Actor%20Object%20Reference) (OtherComp :type Primitive%20Component%20Object%20Reference) (OtherBodyIndex :type Integer) (bFromSweep :type Boolean) (SweepResult :type Hit%20Result%20Structure%20%28by%20ref%29))
  (bind _asbp_game_instance (Utilities|Casting|CastToBP_GameInstance (Game|GetGameInstance))))

(event EventBeginPlay
  (bind _cube (Variables|Default|GetCube))
  (bind _rowname (CallFunction|GetRowNamefromEnum (Variables|Default|GetName)))
  (bind _returnvalue (Utilities|GetDataTableRow "/Game/FunctionPrototyping/Inventory_System/DT_InventoryItem.DT_InventoryItem" _rowname)
    (:then
      (if true
        (Components|StaticMesh|SetStaticMesh _cube (.StaticMesh (Utilities|Struct|BreakS_InventoryItem _returnvalue)))
        (Rendering|Material|SetMaterial _cube 0 (.Material (Utilities|Struct|BreakS_InventoryItem _returnvalue)))))))

(fn ConstructionScript)

(fn GetRowNamefromEnum
  (params (ItemName :type E_ItemName%20Enum :default "NewEnumerator0"))
  (switch Utilities|FlowControl|Switch|SwitchonE_ItemName ItemName
    (:NewEnumerator0
      (return (Utilities|Name|MakeLiteralName "Grass")))
    (:NewEnumerator1
      (return (Utilities|Name|MakeLiteralName "Rock")))))